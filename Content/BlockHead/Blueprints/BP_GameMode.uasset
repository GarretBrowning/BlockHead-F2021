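; Game mode for BlockHead that controls level progression and the end-of-game screens.
; On begin play it sets game-only input, adds the HUD and parses the current level number from the map name.
; LevelComplete shows a widget, then a timer opens the next numbered level or, on the last, the final menu.
; EndGame shows that same menu as a loss, with mouse cursor and UI-only input.
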(event `self.ReceiveBeginPlay`
  (bind _returnvalue (`GameplayStatics.GetPlayerController` 0))
  ;[0.175 1 0.3813] On Begin Play Hide Mouse and Enable Game Only Input
  (set `PlayerController.bShowMouseCursor` false _returnvalue)
  (`WidgetBlueprintLibrary.SetInputMode_GameOnly` _returnvalue)
  ;[0.175 1 0.3813] When Play Begins Add the HUD to the Viewport
  (bind _returnvalue_2 (`|CreateWidget` "/Game/BlockHead/Blueprints/WBP_HUD.WBP_HUD_C"))
  (bind _output_get (set `self.WPB_HUD` _returnvalue_2))
  (`UserWidget.AddToViewport` _output_get 0)
  ;[0.175 1 0.3813] Extract Level Number From Level Name
  (bind _returnvalue_3 (`GameplayStatics.GetCurrentLevelName` true))
  (set `self.CurrentLevel` (`KismetStringLibrary.Conv_StringToInt` (`|GetArrayItem` (`KismetStringLibrary.ParseIntoArray` _returnvalue_3 "Level")))))

(fn `EndGame`
  (`self.LoadFinalMenu` false))

(fn `levelComplete`
  ;[0.175 1 0.3813] Display the "Level Complete" WBP. Delay for 2 seconds and then call LoadNextLevel Function.
  (bind _returnvalue (`|CreateWidget` "/Game/BlockHead/Blueprints/WBP_LevelComplete.WBP_LevelComplete_C"))
  (bind _output_get (set `self.WBP_LevelComplete` _returnvalue))
  (`UserWidget.AddToViewport` _output_get 0)
  (`KismetSystemLibrary.K2_SetTimer` null "LoadNextLevel" 2.0))

(fn `LoadFinalMenu`
  (params (bGameWon :type Boolean))
  (bind _returnvalue (`GameplayStatics.GetPlayerController` 0))
  ;[0.175 1 0.3813] What Text Should be Used in the Game Complete Widget?
  (if bGameWon
    (set `self.FinalMenuText` "Game Complete! :)")
    (else
      (set `self.FinalMenuText` "Game Over! :(")))
  ;[0.175 1 0.3813] Load Game Complete WBP and Set the Win/Loss Text
  (bind _returnvalue_2 (`|CreateWidget` "/Game/BlockHead/Blueprints/WBP_GameCompleted.WBP_GameCompleted_C"))
  (bind _output_get (set `self.GameCompleteWBP` _returnvalue_2))
  (`TextBlock.SetText` (`/Game/BlockHead/Blueprints/WBP_GameCompleted.LostOrComplete` _output_get) (`KismetTextLibrary.Conv_StringToText` (`self.FinalMenuText`)))
  ;[0.175 1 0.3813] Add Game Complete WBP to Viewport. Show Mouse. Set Input Mode to UI Only.
  (`UserWidget.AddToViewport` (`self.GameCompleteWBP`) 0)
  (set `PlayerController.bShowMouseCursor` true _returnvalue)
  (`WidgetBlueprintLibrary.SetInputMode_UIOnlyEx` _returnvalue null))

(fn `LoadNextLevel`
  (bind _wbp_levelcomplete (`self.WBP_LevelComplete`))
  ;[0.175 1 0.3813] Are we already on the final level? Yes means True.
  (if (== (`self.MaxLevel`) (`self.CurrentLevel`))
    ;[0.175 1 0.3813] Game is Over. Load Final WBP.
    (`self.LoadFinalMenu` true)
    (else
      ;[0.175 1 0.3813] Load the Next Level
      (`GameplayStatics.OpenLevel` (`KismetStringLibrary.Conv_StringToName` (`KismetStringLibrary.BuildString_Int` "" "Level" (+ (`self.CurrentLevel`) 1))))))
  ;[0.175 1 0.3813] Remove "Level Complete" WBP if it is Loaded
  (if (`KismetSystemLibrary.IsValid` _wbp_levelcomplete)
    (`Widget.RemoveFromParent` _wbp_levelcomplete)))

(fn `UserConstructionScript`)